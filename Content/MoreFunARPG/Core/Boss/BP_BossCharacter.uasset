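; Boss character with a health bar widget, three attack hitboxes and a montage-driven stun.
; Attack enable events switch on the charge, ranged or melee box from the current state flags, and disabling turns all three off.
; Melee and ranged overlaps share the weapon-hit handler, while charge overlaps have their own.
; Received damage spawns a damage-text widget at the boss's projected screen position, and stun ends when its montage completes.
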(event OnComponentBeginOverlap(MeleeBox)
  (params (OverlappedComponent :type Primitive%20Component%20Object%20Reference) (OtherActor :type Actor%20Object%20Reference) (OtherComp :type Primitive%20Component%20Object%20Reference) (OtherBodyIndex :type Integer) (bFromSweep :type Boolean) (SweepResult :type Hit%20Result%20Structure%20%28by%20ref%29))
  (Class|BossCharacter|OnWeaponOverlap OtherActor))

(event OnComponentBeginOverlap(RangeBox)
  (params (OverlappedComponent :type Primitive%20Component%20Object%20Reference) (OtherActor :type Actor%20Object%20Reference) (OtherComp :type Primitive%20Component%20Object%20Reference) (OtherBodyIndex :type Integer) (bFromSweep :type Boolean) (SweepResult :type Hit%20Result%20Structure%20%28by%20ref%29))
  (Class|BossCharacter|OnWeaponOverlap OtherActor))

(event OnComponentBeginOverlap(Charge)
  (params (OverlappedComponent :type Primitive%20Component%20Object%20Reference) (OtherActor :type Actor%20Object%20Reference) (OtherComp :type Primitive%20Component%20Object%20Reference) (OtherBodyIndex :type Integer) (bFromSweep :type Boolean) (SweepResult :type Hit%20Result%20Structure%20%28by%20ref%29))
  (Class|BossCharacter|OnChargeOverlap OtherActor))

(event Custom|DamageReceived_Event_0
  (params (Damage :type Integer))
  (bind _returnvalue (UserInterface|CreateWidget "/Game/MoreFunARPG/Core/UI/WB_DamageText.WB_DamageText_C" 0 Damage))
  (UserInterface|Viewport|AddtoViewport _returnvalue 0)
  (Class|UserWidget|SetPositioninViewport _returnvalue (.ScreenPosition (Class|WidgetLayoutLibrary|ProjectWorldLocationtoWidgetPosition (Game|GetPlayerController 0) (Transformation|GetActorLocation) false)) false))

(event Custom|SetupWidget
  (bind _aswb_health_bar (Utilities|Casting|CastToWB_HealthBar (UserInterface|GetUserWidgetObject (Variables|Default|GetHealthBar))))
  (Variables|/Game/MoreFunARPG/Core/UI/WB_HealthBar.WB_HealthBar_C|SetOwner _aswb_health_bar self))

(event Custom|SetupDelegate
  (EventDispatchers|AssignDamageReceived (delegate Custom|DamageReceived_Event_0)))

(event Custom|DisableAttackBox
  (Class|BossCharacter|DisableWeapon (Variables|Default|GetMeleeBox))
  (Class|BossCharacter|DisableWeapon (Variables|Default|GetRangeBox))
  (Class|BossCharacter|DisableWeapon (Variables|Default|GetCharge)))

(event EventBeginPlay
  (CallFunction|SetupWidget)
  (CallFunction|SetupDelegate)
  (CallFunction|DisableAttackBox))

(event Collision|EventActorBeginOverlap
  (params (OtherActor :type Actor%20Object%20Reference)))

(event EventTick
  (params (DeltaSeconds :type Float%20%28single-precision%29)))

(event EventOnStun
  (bind _returnvalue (Class|BossCharacter|BeginStun))
  (if _returnvalue
    (Animation|Montage|PlayMontage (Variables|Character|GetMesh) "/Game/MoreFunARPG/Core/Boss/Montage/AM_Stun.AM_Stun" 1.0 0.0 "Default"
      (:OnCompleted
        (Class|BossCharacter|EndStun)))))

(event EventAttackEnabled
  (if (Variables|Default|GetbIsCharging)
    (Class|BossCharacter|EnableWeapon (Variables|Default|GetCharge))
    (elif (Variables|Default|GetbIsRangeAttacking)
      (Class|BossCharacter|EnableWeapon (Variables|Default|GetRangeBox))
      (else
        (Class|BossCharacter|EnableWeapon (Variables|Default|GetMeleeBox))))))

(event EventAttackDiabled
  (CallFunction|DisableAttackBox))

(fn ConstructionScript)