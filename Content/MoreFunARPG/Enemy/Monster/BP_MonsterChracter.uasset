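; Monster enemy character for an action RPG, with a health bar widget, hit reactions, a melee hitbox and a heal trigger.
; Damage events spawn floating damage text at the monster's projected screen position.
; OnHit plays a reaction montage when BeginOnHit allows it, while also opening a timed invincibility window.
; Attack events toggle the HitBox, whose overlaps feed OnWeaponOverlap.
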(event OnComponentBeginOverlap(HitBox)
  (params (OverlappedComponent :type Primitive%20Component%20Object%20Reference) (OtherActor :type Actor%20Object%20Reference) (OtherComp :type Primitive%20Component%20Object%20Reference) (OtherBodyIndex :type Integer) (bFromSweep :type Boolean) (SweepResult :type Hit%20Result%20Structure%20%28by%20ref%29))
  (Class|MonsterCharacter|OnWeaponOverlap OtherActor))

(event Custom|DamageReceived_Event_0
  (params (Damage :type Integer))
  (bind _returnvalue (UserInterface|CreateWidget "/Game/MoreFunARPG/UI/WB_DamageText.WB_DamageText_C" 0 Damage))
  (UserInterface|Viewport|AddtoViewport _returnvalue 0)
  (Class|UserWidget|SetPositioninViewport _returnvalue (.ScreenPosition (Class|WidgetLayoutLibrary|ProjectWorldLocationtoWidgetPosition (Game|GetPlayerController 0) (Transformation|GetActorLocation) false)) false))

(event Custom|SetupWidget
  (bind _aswb_health_bar (Utilities|Casting|CastToWB_HealthBar (UserInterface|GetUserWidgetObject (Variables|Default|GetHealthBar))))
  (Variables|/Game/MoreFunARPG/UI/WB_HealthBar.WB_HealthBar_C|SetOwner _aswb_health_bar self))

(event Custom|SetupDelegate
  (EventDispatchers|AssignDamageReceived (delegate Custom|DamageReceived_Event_0)))

(event EventBeginPlay
  (CallFunction|SetupWidget)
  (Class|MonsterCharacter|DisableWeapon (Variables|Default|GetHitBox))
  (CallFunction|SetupDelegate))

(event Collision|EventActorBeginOverlap
  (params (OtherActor :type Actor%20Object%20Reference)))

(event EventTick
  (params (DeltaSeconds :type Float%20%28single-precision%29)))

(event EventOnHit
  (bind _returnvalue (Class|MonsterCharacter|BeginonHit))
  (Utilities|FlowControl|Sequence
    (:then_0
      (if _returnvalue
        (Animation|Montage|PlayMontage (Variables|Character|GetMesh) "/Game/MoreFunARPG/Enemy/Monster/Montage/AM_OnHit.AM_OnHit" 1.0 0.0 "Default"
          (:OnCompleted
            (Class|MonsterCharacter|EndonHit)))))
    (:then_1
      (Class|MonsterCharacter|BeginInvincible)
      (Utilities|FlowControl|Delay (Variables|Default|GetDefaultInvincibleTime))
      (Class|MonsterCharacter|EndInvincible))))

(event EventTriggerHeal
  (Class|MonsterCharacter|ReceiveHeal))

(event EventAttackDiabled
  (Class|MonsterCharacter|DisableWeapon (Variables|Default|GetHitBox)))

(event EventAttackEnabled
  (Class|MonsterCharacter|EnableWeapon (Variables|Default|GetHitBox)))

(fn ConstructionScript)