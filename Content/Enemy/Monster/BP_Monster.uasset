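; Monster enemy Blueprint that wires up the health bar, hit reaction and hitbox overlap.
; On BeginPlay it sets itself as the Owner of its WB_HealthBar widget.
; OnHit plays the AM_OnHit montage if BeginOnHit allows it, calling EndOnHit only when the montage completes, with no interruption handler.
; HitBox overlaps forward the other actor to OnWeaponOverlap, which, like BeginOnHit and EndOnHit, is defined outside these graphs.
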(event OnComponentBeginOverlap(HitBox)
  (params (OverlappedComponent :type Primitive%20Component%20Object%20Reference) (OtherActor :type Actor%20Object%20Reference) (OtherComp :type Primitive%20Component%20Object%20Reference) (OtherBodyIndex :type Integer) (bFromSweep :type Boolean) (SweepResult :type Hit%20Result%20Structure%20%28by%20ref%29))
  (Class|ARPGCharacter|OnWeaponOverlap OtherActor))

(event EventBeginPlay
  (bind _aswb_health_bar (Utilities|Casting|CastToWB_HealthBar (UserInterface|GetUserWidgetObject (Variables|Default|GetHealthBar))))
  (Variables|/Game/UI/WB_HealthBar.WB_HealthBar_C|SetOwner _aswb_health_bar self))

(event Collision|EventActorBeginOverlap
  (params (OtherActor :type Actor%20Object%20Reference)))

(event EventTick
  (params (DeltaSeconds :type Float%20%28single-precision%29)))

(event EventOnHit
  (bind _returnvalue (Class|MonsterCharacter|BeginonHit))
  (if _returnvalue
    (Animation|Montage|PlayMontage (Variables|Character|GetMesh) "/Game/Enemy/Monster/Montage/AM_OnHit.AM_OnHit" 1.0 0.0 "Default"
      (:OnCompleted
        (Class|MonsterCharacter|EndonHit)))))

(fn ConstructionScript)