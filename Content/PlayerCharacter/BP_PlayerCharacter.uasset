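; Player character Blueprint that drives combo attacks, rolling, running, healing and hit reactions.
; Begin/End calls gate each action, with montages supplying animation; the combo index selects the attack section.
; Weapon events toggle the HitBox, whose overlaps go to OnWeaponOverlap.
; Rolls and hits grant invincibility, whose events drive a looping timer that cycles emissive mesh colors; T is a test damage key.
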(event OnComponentBeginOverlap(HitBox)
  (params (OverlappedComponent :type Primitive%20Component%20Object%20Reference) (OtherActor :type Actor%20Object%20Reference) (OtherComp :type Primitive%20Component%20Object%20Reference) (OtherBodyIndex :type Integer) (bFromSweep :type Boolean) (SweepResult :type Hit%20Result%20Structure%20%28by%20ref%29))
  ;[1 1 1] Battle Event
  (Class|ARPGCharacter|OnWeaponOverlap OtherActor))

(event Custom|PlayHitEffect
  (bind _mesh (Variables|Character|GetMesh))
  ;[1 1 1] Hit Effect
  (Utilities|FlowControl|FlipFlop
    (:A
      (Utilities|FlowControl|FlipFlop
        (:A
          (Variables|Default|SetHitColor "(R=1.000000,G=0.000000,B=0.115404,A=1.000000)"))
        (:B
          (Variables|Default|SetHitColor "(R=0.000000,G=0.923441,B=1.000000,A=1.000000)"))))
    (:B
      (Utilities|FlowControl|FlipFlop
        (:A
          (Variables|Default|SetHitColor "(R=1.000000,G=0.440653,B=0.000000,A=1.000000)"))
        (:B
          (Variables|Default|SetHitColor "(R=0.000000,G=1.000000,B=0.164729,A=1.000000)")))))
  (Rendering|Material|SetVectorParameterValueonMaterials _mesh "EmitColor" (Math|Conversions|ToVector(LinearColor) (Variables|Default|GetHitColor)))
  (Rendering|Material|SetScalarParameterValueonMaterials _mesh "Intensity" 1.0))

(event Custom|StopHitEffect
  ;[1 1 1] Hit Effect
  (Rendering|Material|SetScalarParameterValueonMaterials (Variables|Character|GetMesh) "Intensity" 0.0))

(event EventBeginPlay
  (Class|PlayerCharacter|DisableWeapon (Variables|Default|GetHitBox)))

(event EventAttackUnlock
  ;[1 1 1] Battle Event
  (Class|PlayerCharacter|EndPrimaryAttack))

(event EventOnPrimaryAttackPressed
  ;[1 1 1] Input Bind Blueprint Implementation
  (bind (_outcomboanimindex _returnvalue) (Class|PlayerCharacter|BeginPrimaryAttack))
  (if _returnvalue
    (switch int _outcomboanimindex
      (:0
        (Variables|Default|SetComboSectionName "First"))
      (:1
        (Variables|Default|SetComboSectionName "Second"))
      (:2
        (Variables|Default|SetComboSectionName "Third"))
      (:3
        (Variables|Default|SetComboSectionName "Forth")))
    (Animation|Montage|PlayMontage (Variables|Character|GetMesh) "/Game/PlayerCharacter/Montage/AM_ComboAttack.AM_ComboAttack" 1.0 0.0 (Variables|Default|GetComboSectionName))))

(event EventOnRollPressed
  ;[1 1 1] Input Bind Blueprint Implementation
  (bind _returnvalue (Class|PlayerCharacter|BeginRolling))
  (if _returnvalue
    (Class|PlayerCharacter|BeginInvincible)
    (Animation|Montage|PlayMontage (Variables|Character|GetMesh) "/Game/PlayerCharacter/Montage/AM_PlayerRoll.AM_PlayerRoll" 1.0 0.0 "Default"
      (:OnCompleted
        (Class|PlayerCharacter|EndRolling)
        (Class|PlayerCharacter|EndInvincible)))))

(event EventOnHealPressed
  ;[1 1 1] Input Bind Blueprint Implementation
  (bind _returnvalue (Class|PlayerCharacter|BeginHealing))
  (if _returnvalue
    (Animation|Montage|PlayMontage (Variables|Character|GetMesh) "/Game/PlayerCharacter/Montage/AM_Heal.AM_Heal" 1.0 0.0 "Default"
      (:OnCompleted
        (Class|PlayerCharacter|EndHealing)))))

(event EventOnInvincibleBegin
  ;[1 1 1] Battle Event
  (Utilities|Time|SetTimerbyFunctionName 0 "PlayHitEffect" 0.025 true))

(event EventOnInvincibleEnd
  ;[1 1 1] Battle Event
  (Utilities|Time|ClearTimerbyFunctionName self "PlayHitEffect")
  (CallFunction|StopHitEffect))

(event EventTriggerHeal
  ;[1 1 1] Battle Event
  (Class|PlayerCharacter|ReceiveHeal))

(event EventAttackDiabled
  ;[1 1 1] Battle Event
  (Class|PlayerCharacter|DisableWeapon (Variables|Default|GetHitBox)))

(event EventAttackEnabled
  ;[1 1 1] Battle Event
  (Class|PlayerCharacter|EnableWeapon (Variables|Default|GetHitBox)))

(event EventOnHit
  ;[1 1 1] Battle Event
  (bind _returnvalue (Class|PlayerCharacter|BeginonHit))
  (Utilities|FlowControl|Sequence
    (:then_0
      (if _returnvalue
        (Animation|Montage|PlayMontage (Variables|Character|GetMesh) "/Game/PlayerCharacter/Montage/AM_Hit.AM_Hit"
          (:OnCompleted
            (Class|PlayerCharacter|EndonHit)))))
    (:then_1
      (Class|PlayerCharacter|BeginInvincible)
      (Utilities|FlowControl|Delay (Variables|Default|GetDefaultInvincibleTime))
      (Class|PlayerCharacter|EndInvincible))))

(event EventOnRunningPressed
  ;[1 1 1] Input Bind Blueprint Implementation
  (Class|PlayerCharacter|BeginRunning))

(event EventOnRunningReleased
  ;[1 1 1] Input Bind Blueprint Implementation
  (Class|PlayerCharacter|EndRunning))

(event Input|KeyboardEvents|T
  (params (Key :type Key%20Structure :default "None"))
  ;[1 1 1] Test
  (:Pressed
    (Class|PlayerCharacter|ReceiveDamage 40)))

(fn ConstructionScript)