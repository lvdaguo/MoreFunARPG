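; Player controller that forwards movement, look, running, attack, roll and heal input to the possessed PlayerCharacter, cached on BeginPlay.
; Attack, roll and heal play montages on the character mesh only when the character's Begin call succeeds; the combo index picks the attack section.
; Roll and heal call their End functions on montage completion.
; J, T and Y are test keys for experience, damage and healing; UnPossess disables the pawn's input.
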(event EventBeginPlay
  (bind _asplayer_character (Utilities|Casting|CastToPlayerCharacter (Pawn|GetControlledPawn)))
  (Variables|Default|SetPlayerCharacter _asplayer_character)
  (Variables|Default|SetPlayerMesh (Variables|/Script/Engine.Character|GetMesh _asplayer_character)))

(event EventTick
  (params (DeltaSeconds :type Float%20%28single-precision%29)))

(event EventUnPossess
  (params (UnpossessedPawn :type Pawn%20Object%20Reference))
  (Development|PrintString "ahaha")
  (Input|DisableInput UnpossessedPawn self))

(event Input|ActionEvents|InputActionRoll
  (params (Key :type Key%20Structure :default "None"))
  (:Pressed
    (bind _returnvalue (Class|PlayerCharacter|BeginRolling (Variables|Default|GetPlayerCharacter)))
    (if _returnvalue
      (Animation|Montage|PlayMontage (Variables|Default|GetPlayerMesh) "/Game/PlayerCharacter/Montage/AM_PlayerRoll.AM_PlayerRoll" 1.0 0.0 "Default"
        (:OnCompleted
          (Class|PlayerCharacter|EndRolling (Variables|Default|GetPlayerCharacter)))))))

(event Input|ActionEvents|InputActionPrimaryAttack
  (params (Key :type Key%20Structure :default "None"))
  (:Pressed
    (bind (_outcomboanimindex _returnvalue) (Class|PlayerCharacter|BeginPrimaryAttack (Variables|Default|GetPlayerCharacter)))
    (if _returnvalue
      (switch int _outcomboanimindex
        (:0
          (Variables|Default|SetComboSectionName "First"))
        (:1
          (Variables|Default|SetComboSectionName "Second"))
        (:2
          (Variables|Default|SetComboSectionName "Third"))
        (:3
          (Variables|Default|SetComboSectionName "Forth")))
      (Animation|Montage|PlayMontage (Variables|Default|GetPlayerMesh) "/Game/PlayerCharacter/Montage/AM_ComboAttack.AM_ComboAttack" 1.0 0.0 (Variables|Default|GetComboSectionName)))))

(event Input|ActionEvents|InputActionHeal
  (params (Key :type Key%20Structure :default "None"))
  (:Pressed
    (bind _returnvalue (Class|PlayerCharacter|BeginHealing (Variables|Default|GetPlayerCharacter)))
    (if _returnvalue
      (Animation|Montage|PlayMontage (Variables|Default|GetPlayerMesh) "/Game/PlayerCharacter/Montage/AM_Heal.AM_Heal" 1.0 0.0 "Default"
        (:OnCompleted
          (Class|PlayerCharacter|EndHealing (Variables|Default|GetPlayerCharacter)))))))

(event Input|ActionEvents|InputActionRunning
  (params (Key :type Key%20Structure :default "None"))
  (bind _playercharacter (Variables|Default|GetPlayerCharacter))
  (:Pressed
    (Class|PlayerCharacter|BeginRunning _playercharacter))
  (:Released
    (Class|PlayerCharacter|EndRunning _playercharacter)))

(event Input|AxisEvents|InputAxisMoveForward
  (params (AxisValue :type Float%20%28single-precision%29))
  ;[1 1 1] Bind Axis
  (Class|PlayerCharacter|MoveForward (Variables|Default|GetPlayerCharacter) AxisValue))

(event Input|AxisEvents|InputAxisMoveRight
  (params (AxisValue :type Float%20%28single-precision%29))
  ;[1 1 1] Bind Axis
  (Class|PlayerCharacter|MoveRight (Variables|Default|GetPlayerCharacter) AxisValue))

(event Input|AxisEvents|InputAxisLookUp
  (params (AxisValue :type Float%20%28single-precision%29))
  ;[1 1 1] Bind Axis
  (Class|PlayerCharacter|LookUp (Variables|Default|GetPlayerCharacter) AxisValue))

(event Input|AxisEvents|InputAxisTurn
  (params (AxisValue :type Float%20%28single-precision%29))
  ;[1 1 1] Bind Axis
  (Class|PlayerCharacter|Turn (Variables|Default|GetPlayerCharacter) AxisValue))

(event Input|KeyboardEvents|J
  (params (Key :type Key%20Structure :default "None"))
  ;[1 1 1] Test
  (:Pressed
    (Class|PlayerCharacter|ReceiveExp (Variables|Default|GetPlayerCharacter) 200)))

(event Input|KeyboardEvents|T
  (params (Key :type Key%20Structure :default "None"))
  ;[1 1 1] Test
  (:Pressed
    (Class|PlayerCharacter|ReceiveDamage (Variables|Default|GetPlayerCharacter) 40)))

(event Input|KeyboardEvents|Y
  (params (Key :type Key%20Structure :default "None"))
  ;[1 1 1] Test
  (:Pressed
    (Class|ARPGCharacter|ReceiveHeal (Variables|Default|GetPlayerCharacter) 10)))

(fn ConstructionScript)